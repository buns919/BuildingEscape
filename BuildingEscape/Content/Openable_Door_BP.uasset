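; Openable door actor that responds to OpenDoor open and close events by swinging on its yaw axis.
; The DoorSwing timeline plays forward or in reverse, setting the actor's absolute rotation from its OpenAngle track.
; A Sound Timing event track on the timeline plays the door lock sound at the actor's location.
; BeginPlay stores InitialRotation and clears DoorIsOpen, but the swing logic uses neither.
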(event OnOpen(OpenDoor)
  (bind _open_angle (Timeline|Door%20Swing Play)
    (:Update
      (Transformation|SetActorRotation (Math|Rotator|MakeRotator 0.0 0.0 _open_angle)))
    (:Sound%20Timing
      (CallFunction|PlayDoorSoundatLocation))))

(event OnClose(OpenDoor)
  (bind _open_angle (Timeline|Door%20Swing Reverse)
    (:Update
      (Transformation|SetActorRotation (Math|Rotator|MakeRotator 0.0 0.0 _open_angle)))
    (:Sound%20Timing
      (CallFunction|PlayDoorSoundatLocation))))

(event EventBeginPlay
  (Variables|Default|SetbDoorIsOpen false)
  (Variables|Default|SetInitialRotation (Transformation|GetActorRotation)))

(fn ConstructionScript)

(fn PlayDoorSoundatLocation
  (Audio|PlaySoundatLocation "/Game/Audio/door-lock.door-lock" (Transformation|GetActorLocation) "0, 0, 0" 1.0 1.0 0.0 0 0 0))